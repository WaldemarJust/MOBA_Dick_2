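; Game mode for a MOBA-style match that spawns lane minions and jungle monsters and respawns the player character after death.
; BeginPlay sorts waypoints into five lanes per team, reversing team 1's order, and caches spawn points by minion type.
; A wave timer, capped by live minion count, resets DoN gates that a one-second timer drains into staggered spawns.
; Jungle monsters spawn once after a delay, and the player's destruction triggers respawn and possession.
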(event Custom|OnDestroyed_Event_0
  (params (DestroyedActor :type Actor%20Object%20Reference))
  (Utilities|FlowControl|Delay 1.0)
  (CallFunction|RespawnCharakter))

(event Custom|Respawn
  (bind _asmage_bp (Utilities|Casting|CastToMage_BP (Game|GetPlayerCharacter 0)))
  (Game|BindEventtoOnDestroyed _asmage_bp (delegate Custom|OnDestroyed_Event_0)))

(event Custom|SpawnWavePart1
  (Utilities|FlowControl|Sequence
    (:then_0
      (Utilities|FlowControl|DoN 3
        (:Exit
          (CallFunction|SapwnMinionLandMelee)
          (CallFunction|SapwnMinionWaterMelee)
          (CallFunction|SapwnMinion))))
    (:then_1
      (Utilities|FlowControl|DoN 2
        (:Exit
          (CallFunction|SapwnMinionLandRanged)
          (CallFunction|SapwnMinionWaterRanged))))))

(event Custom|OnDestroyed_Event_1
  (params (DestroyedActor :type Actor%20Object%20Reference))
  (Utilities|FlowControl|Delay 5.0)
  (Utilities|FlowControl|DoOnce false) ; enters at Reset
)

(event Custom|Spawn%20Minion%20Wave
  (bind _outactors (Actor|GetAllActorsOfClass "/Game/Minions/Units/Minion.Minion_C"))
  (if (<= (Utilities|Array|Length _outactors) 50)
    (Utilities|FlowControl|Sequence
      (:then_0
        (Utilities|FlowControl|DoN 3) ; enters at Reset
      )
      (:then_1
        (Utilities|FlowControl|DoN 2) ; enters at Reset
      ))))

(event EventBeginPlay
  (bind _waypiontcount (Variables|Default|GetWaypiontCount))
  (bind _waypiontcount_2 (Variables|Default|GetWaypiontCount))
  (Utilities|FlowControl|Sequence
    (:then_0
      (bind _outactors (Actor|GetAllActorsOfClass "/Game/Minions/Actors/Waypoint.Waypoint_C"))
      (Utilities|Array|Clear _waypiontcount)
      (Utilities|Array|Resize _waypiontcount 5)
      (for _array_element _outactors
        (Utilities|Array|SetArrayElem _waypiontcount_2 (Variables|/Game/Minions/Actors/Waypoint.Waypoint_C|GetLane _array_element) (+ (Utilities|Array|Get(acopy) _waypiontcount_2 (Variables|/Game/Minions/Actors/Waypoint.Waypoint_C|GetLane _array_element)) 1)))
      (for _array_element_2 _outactors
        (switch int (Variables|/Game/Minions/Actors/Waypoint.Waypoint_C|GetLane _array_element_2)
          (:0
            (Utilities|Array|SetArrayElem (Variables|Default|GetTeam0Lane0) (Variables|/Game/Minions/Actors/Waypoint.Waypoint_C|GetWaypiontNumber _array_element_2) _array_element_2 true)
            (Utilities|Array|SetArrayElem (Variables|Default|GetTeam1Lane0) (- (- (Utilities|Array|Get(acopy) (Variables|Default|GetWaypiontCount) (Variables|/Game/Minions/Actors/Waypoint.Waypoint_C|GetLane _array_element_2)) 1) (Variables|/Game/Minions/Actors/Waypoint.Waypoint_C|GetWaypiontNumber _array_element_2)) _array_element_2 true))
          (:1
            (Utilities|Array|SetArrayElem (Variables|Default|GetTeam0Lane1) (Variables|/Game/Minions/Actors/Waypoint.Waypoint_C|GetWaypiontNumber _array_element_2) _array_element_2 true)
            (Utilities|Array|SetArrayElem (Variables|Default|GetTeam1Lane1) (- (- (Utilities|Array|Get(acopy) (Variables|Default|GetWaypiontCount) (Variables|/Game/Minions/Actors/Waypoint.Waypoint_C|GetLane _array_element_2)) 1) (Variables|/Game/Minions/Actors/Waypoint.Waypoint_C|GetWaypiontNumber _array_element_2)) _array_element_2 true))
          (:2
            (Utilities|Array|SetArrayElem (Variables|Default|GetTeam0Lane2) (Variables|/Game/Minions/Actors/Waypoint.Waypoint_C|GetWaypiontNumber _array_element_2) _array_element_2 true)
            (Utilities|Array|SetArrayElem (Variables|Default|GetTeam1Lane2) (- (- (Utilities|Array|Get(acopy) (Variables|Default|GetWaypiontCount) (Variables|/Game/Minions/Actors/Waypoint.Waypoint_C|GetLane _array_element_2)) 1) (Variables|/Game/Minions/Actors/Waypoint.Waypoint_C|GetWaypiontNumber _array_element_2)) _array_element_2 true))
          (:3
            (Utilities|Array|SetArrayElem (Variables|Default|GetTeam0Lane3) (Variables|/Game/Minions/Actors/Waypoint.Waypoint_C|GetWaypiontNumber _array_element_2) _array_element_2 true)
            (Utilities|Array|SetArrayElem (Variables|Default|GetTeam1Lane3) (- (- (Utilities|Array|Get(acopy) (Variables|Default|GetWaypiontCount) (Variables|/Game/Minions/Actors/Waypoint.Waypoint_C|GetLane _array_element_2)) 1) (Variables|/Game/Minions/Actors/Waypoint.Waypoint_C|GetWaypiontNumber _array_element_2)) _array_element_2 true))
          (:4
            (Utilities|Array|SetArrayElem (Variables|Default|GetTeam0Lane4) (Variables|/Game/Minions/Actors/Waypoint.Waypoint_C|GetWaypiontNumber _array_element_2) _array_element_2 true)
            (Utilities|Array|SetArrayElem (Variables|Default|GetTeam1Lane4) (- (- (Utilities|Array|Get(acopy) (Variables|Default|GetWaypiontCount) (Variables|/Game/Minions/Actors/Waypoint.Waypoint_C|GetLane _array_element_2)) 1) (Variables|/Game/Minions/Actors/Waypoint.Waypoint_C|GetWaypiontNumber _array_element_2)) _array_element_2 true)))))
    (:then_1
      (Utilities|FlowControl|Sequence
        (:then_0
          (bind _outactors_2 (Actor|GetAllActorsOfClass "/Game/Minions/Actors/MinionSpawnPiont.MinionSpawnPiont_C"))
          (Variables|Default|SetMinionSpawns _outactors_2))
        (:then_1
          (bind _outactors_3 (Actor|GetAllActorsOfClass "/Game/Minions/Actors/MinionSpawnPiont_LandMelee.MinionSpawnPiont_LandMelee_C"))
          (Variables|Default|SetMinionSpawns_LandMelee _outactors_3))
        (:then_2
          (bind _outactors_4 (Actor|GetAllActorsOfClass "/Game/Minions/Actors/MinionSpawnPiont_LandRanged.MinionSpawnPiont_LandRanged_C"))
          (Variables|Default|SetMinionSpawns_LandRanged _outactors_4))
        (:then_3
          (bind _outactors_5 (Actor|GetAllActorsOfClass "/Game/Minions/Actors/MinionSpawnPiont_WaterMelee.MinionSpawnPiont_WaterMelee_C"))
          (Variables|Default|SetMinionSpawns_WaterMelee _outactors_5))
        (:then_4
          (bind _outactors_6 (Actor|GetAllActorsOfClass "/Game/Minions/Actors/MinionSpawnPiont_WaterRanged.MinionSpawnPiont_WaterRanged_C"))
          (Variables|Default|SetMinionSpawns_WaterRanged _outactors_6))
        (:then_5
          (bind _outactors_7 (Actor|GetAllActorsOfClass "/Game/Minions/Actors/MinionSpawnPiont_MOBA_DICK.MinionSpawnPiont_MOBA_DICK_C"))
          (Variables|Default|SetMinionSpawns_MOBA_DICK _outactors_7))
        (:then_6
          (bind _outactors_8 (Actor|GetAllActorsOfClass "/Game/Minions/Actors/MinionSpawnPiont_JungleWolfBig.MinionSpawnPiont_JungleWolfBig_C"))
          (Variables|Default|SetMinionSpawns_JungleWolfBig _outactors_8))
        (:then_7
          (bind _outactors_9 (Actor|GetAllActorsOfClass "/Game/Minions/Actors/MinionSpawnPiont_JungleWolfSmall.MinionSpawnPiont_JungleWolfSmall_C"))
          (Variables|Default|SetMinionSpawns_JungleWolfSmall _outactors_9))))
    (:then_2
      (Utilities|FlowControl|Delay 1.0)
      (Utilities|Time|SetTimerbyEvent (delegate Custom|SpawnWavePart1) 1.0 true)
      (Utilities|Time|SetTimerbyEvent (delegate Custom|Spawn%20Minion%20Wave) (Variables|Default|GetWaveSpawnTime) true))
    (:then_3
      (bind _asmage_bp (Utilities|Casting|CastToMage_BP (Game|GetPlayerCharacter 0)))
      (Game|BindEventtoOnDestroyed _asmage_bp (delegate Custom|OnDestroyed_Event_0)))
    (:then_4
      (Utilities|FlowControl|Delay 3e+01)
      (Utilities|FlowControl|Sequence
        (:then_0
          (Utilities|FlowControl|DoOnce false
            (:Completed
              (CallFunction|SapwnMinionMOBADICK))))
        (:then_1
          (Utilities|FlowControl|DoOnce false
            (:Completed
              (CallFunction|SapwnMinionJungleWolfBig))))
        (:then_2
          (Utilities|FlowControl|DoOnce false
            (:Completed
              (CallFunction|SapwnMinionJungleWolfSmall))))))))

(event EventDestroyed
  (bind _asminion_moba_dick (Utilities|Casting|CastToMinion_MOBA_DICK (Components|GetOwner))
    (:then
      (Game|AssignOnDestroyed _asminion_moba_dick (delegate Custom|OnDestroyed_Event_1)))
    (:CastFailed
      (Development|PrintString "not moba dick"))))

(fn ConstructionScript)

(fn RespawnCharakter
  (bind _returnvalue (Game|SpawnActorfromClass "/Game/Blueprints/MyCharacter.MyCharacter_C" (Variables|Default|GetSpawnTransform) "Undefined" 0 0))
  (Pawn|Possess (Game|GetPlayerController 0) _returnvalue)
  (CallFunction|Respawn)
  (return))

(fn GetWaypionsforMinions
  (params (Team :type Integer) (Lane :type Integer))
  (return (Utilities|Select :Index (+ (* Team 5) Lane) :Option%200 (Variables|Default|GetTeam0Lane0) :Option%201 (Variables|Default|GetTeam0Lane1) :Option%202 (Variables|Default|GetTeam0Lane2) :Option%203 (Variables|Default|GetTeam0Lane3) :Option%204 (Variables|Default|GetTeam0Lane4) :Option%205 (Variables|Default|GetTeam1Lane0) :Option%206 (Variables|Default|GetTeam1Lane1) :Option%207 (Variables|Default|GetTeam1Lane2) :Option%208 (Variables|Default|GetTeam1Lane3) :Option%209 (Variables|Default|GetTeam1Lane4))))

(fn SapwnMinion
  (bind _minionspawns (Variables|Default|GetMinionSpawns))
  (for _index (range 0 (Utilities|Array|LastIndex _minionspawns))
    (bind _returnvalue (Game|SpawnActorfromClass "/Game/Minions/Units/Minion.Minion_C" (Math|Transform|MakeTransform (.location (Transformation|GetActorTransform (Utilities|Array|Get(acopy) _minionspawns _index))) (.rotation (Transformation|GetActorTransform (Utilities|Array|Get(acopy) _minionspawns _index))) "1,1,1") "AlwaysSpawn" 0 (Variables|/Game/Minions/Actors/MinionSpawnPiont.MinionSpawnPiont_C|GetTeam (Utilities|Array|Get(acopy) _minionspawns _index)) (Variables|/Game/Minions/Actors/MinionSpawnPiont.MinionSpawnPiont_C|GetLane (Utilities|Array|Get(acopy) _minionspawns _index))))
    (Utilities|Array|Add (Variables|Default|GetMinionArray) _returnvalue)))

(fn SapwnMinionLandMelee
  (bind _minionspawns_landmelee (Variables|Default|GetMinionSpawns_LandMelee))
  (for _index (range 0 (Utilities|Array|LastIndex _minionspawns_landmelee))
    (bind _returnvalue (Game|SpawnActorfromClass "/Game/Minions/Units/Minion_LandMelee.Minion_LandMelee_C" (Math|Transform|MakeTransform (.location (Transformation|GetActorTransform (Utilities|Array|Get(acopy) _minionspawns_landmelee _index))) (.rotation (Transformation|GetActorTransform (Utilities|Array|Get(acopy) _minionspawns_landmelee _index))) "1,1,1") "AlwaysSpawn" 0 (Variables|/Game/Minions/Actors/MinionSpawnPiont.MinionSpawnPiont_C|GetTeam (Utilities|Array|Get(acopy) _minionspawns_landmelee _index)) (Variables|/Game/Minions/Actors/MinionSpawnPiont.MinionSpawnPiont_C|GetLane (Utilities|Array|Get(acopy) _minionspawns_landmelee _index))))
    (Utilities|Array|Add (Variables|Default|GetMinionArray) _returnvalue)))

(fn SapwnMinionLandRanged
  (bind _minionspawns_landranged (Variables|Default|GetMinionSpawns_LandRanged))
  (for _index (range 0 (Utilities|Array|LastIndex _minionspawns_landranged))
    (bind _returnvalue (Game|SpawnActorfromClass "/Game/Minions/Units/Minion_LandRanged.Minion_LandRanged_C" (Math|Transform|MakeTransform (.location (Transformation|GetActorTransform (Utilities|Array|Get(acopy) _minionspawns_landranged _index))) (.rotation (Transformation|GetActorTransform (Utilities|Array|Get(acopy) _minionspawns_landranged _index))) "1,1,1") "AlwaysSpawn" 0 (Variables|/Game/Minions/Actors/MinionSpawnPiont.MinionSpawnPiont_C|GetTeam (Utilities|Array|Get(acopy) _minionspawns_landranged _index)) (Variables|/Game/Minions/Actors/MinionSpawnPiont.MinionSpawnPiont_C|GetLane (Utilities|Array|Get(acopy) _minionspawns_landranged _index))))
    (Utilities|Array|Add (Variables|Default|GetMinionArray) _returnvalue)))

(fn SapwnMinionWaterMelee
  (bind _minionspawns_watermelee (Variables|Default|GetMinionSpawns_WaterMelee))
  (for _index (range 0 (Utilities|Array|LastIndex _minionspawns_watermelee))
    (bind _returnvalue (Game|SpawnActorfromClass "/Game/Minions/Units/Minion_WaterMelee.Minion_WaterMelee_C" (Math|Transform|MakeTransform (.location (Transformation|GetActorTransform (Utilities|Array|Get(acopy) _minionspawns_watermelee _index))) (.rotation (Transformation|GetActorTransform (Utilities|Array|Get(acopy) _minionspawns_watermelee _index))) "1,1,1") "AlwaysSpawn" 0 (Variables|/Game/Minions/Actors/MinionSpawnPiont.MinionSpawnPiont_C|GetTeam (Utilities|Array|Get(acopy) _minionspawns_watermelee _index)) (Variables|/Game/Minions/Actors/MinionSpawnPiont.MinionSpawnPiont_C|GetLane (Utilities|Array|Get(acopy) _minionspawns_watermelee _index))))
    (Utilities|Array|Add (Variables|Default|GetMinionArray) _returnvalue)))

(fn SapwnMinionWaterRanged
  (bind _minionspawns_waterranged (Variables|Default|GetMinionSpawns_WaterRanged))
  (for _index (range 0 (Utilities|Array|LastIndex _minionspawns_waterranged))
    (bind _returnvalue (Game|SpawnActorfromClass "/Game/Minions/Units/Minion_WaterRanged.Minion_WaterRanged_C" (Math|Transform|MakeTransform (.location (Transformation|GetActorTransform (Utilities|Array|Get(acopy) _minionspawns_waterranged _index))) (.rotation (Transformation|GetActorTransform (Utilities|Array|Get(acopy) _minionspawns_waterranged _index))) "1,1,1") "AlwaysSpawn" 0 (Variables|/Game/Minions/Actors/MinionSpawnPiont.MinionSpawnPiont_C|GetTeam (Utilities|Array|Get(acopy) _minionspawns_waterranged _index)) (Variables|/Game/Minions/Actors/MinionSpawnPiont.MinionSpawnPiont_C|GetLane (Utilities|Array|Get(acopy) _minionspawns_waterranged _index))))
    (Utilities|Array|Add (Variables|Default|GetMinionArray) _returnvalue)))

(fn SapwnMinionMOBADICK
  (bind _minionspawns_moba_dick (Variables|Default|GetMinionSpawns_MOBA_DICK))
  (for _index (range 0 (Utilities|Array|LastIndex _minionspawns_moba_dick))
    (bind _returnvalue (Game|SpawnActorfromClass "/Game/Minions/Units/Minion_MOBA_DICK.Minion_MOBA_DICK_C" (Math|Transform|MakeTransform (.location (Transformation|GetActorTransform (Utilities|Array|Get(acopy) _minionspawns_moba_dick _index))) (.rotation (Transformation|GetActorTransform (Utilities|Array|Get(acopy) _minionspawns_moba_dick _index))) "1,1,1") "AlwaysSpawn" 0 (Variables|/Game/Minions/Actors/MinionSpawnPiont.MinionSpawnPiont_C|GetTeam (Utilities|Array|Get(acopy) _minionspawns_moba_dick _index)) (Variables|/Game/Minions/Actors/MinionSpawnPiont.MinionSpawnPiont_C|GetLane (Utilities|Array|Get(acopy) _minionspawns_moba_dick _index))))
    (Utilities|Array|Add (Variables|Default|GetMinionArray_Jungle) _returnvalue)))

(fn SapwnMinionJungleWolfBig
  (bind _minionspawns_junglewolfbig (Variables|Default|GetMinionSpawns_JungleWolfBig))
  (for _index (range 0 (Utilities|Array|LastIndex _minionspawns_junglewolfbig))
    (bind _returnvalue (Game|SpawnActorfromClass "/Game/Minions/Units/JungleMinions/Minion_JungleWolfBig.Minion_JungleWolfBig_C" (Math|Transform|MakeTransform (.location (Transformation|GetActorTransform (Utilities|Array|Get(acopy) _minionspawns_junglewolfbig _index))) (.rotation (Transformation|GetActorTransform (Utilities|Array|Get(acopy) _minionspawns_junglewolfbig _index))) "1,1,1") "AlwaysSpawn" 0 (Variables|/Game/Minions/Actors/MinionSpawnPiont.MinionSpawnPiont_C|GetTeam (Utilities|Array|Get(acopy) _minionspawns_junglewolfbig _index)) (Variables|/Game/Minions/Actors/MinionSpawnPiont.MinionSpawnPiont_C|GetLane (Utilities|Array|Get(acopy) _minionspawns_junglewolfbig _index))))
    (Utilities|Array|Add (Variables|Default|GetMinionArray_Jungle) _returnvalue)))

(fn SapwnMinionJungleWolfSmall
  (bind _minionspawns_junglewolfsmall (Variables|Default|GetMinionSpawns_JungleWolfSmall))
  (for _index (range 0 (Utilities|Array|LastIndex _minionspawns_junglewolfsmall))
    (bind _returnvalue (Game|SpawnActorfromClass "/Game/Minions/Units/JungleMinions/Minion_JungleWolfSmall.Minion_JungleWolfSmall_C" (Math|Transform|MakeTransform (.location (Transformation|GetActorTransform (Utilities|Array|Get(acopy) _minionspawns_junglewolfsmall _index))) (.rotation (Transformation|GetActorTransform (Utilities|Array|Get(acopy) _minionspawns_junglewolfsmall _index))) "1,1,1") "AlwaysSpawn" 0 (Variables|/Game/Minions/Actors/MinionSpawnPiont.MinionSpawnPiont_C|GetTeam (Utilities|Array|Get(acopy) _minionspawns_junglewolfsmall _index)) (Variables|/Game/Minions/Actors/MinionSpawnPiont.MinionSpawnPiont_C|GetLane (Utilities|Array|Get(acopy) _minionspawns_junglewolfsmall _index))))
    (Utilities|Array|Add (Variables|Default|GetMinionArray_Jungle) _returnvalue)))