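; Turret actor that fires homing projectiles at a Character it sees through PawnSensing and destroys itself when its health runs out.
; A sighting targets the capsule, fires at once and starts a looping one-second timer, with a DoOnce preventing duplicate timers.
; A Character leaving GTFO_Radius clears the timer and resets the DoOnce.
; Damage lowers TurretHealth and updates the HealthBar widget.
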(event OnComponentBeginOverlap(PissOffRadius)
  (params (OverlappedComponent :type Primitive%20Component%20Object%20Reference) (OtherActor :type Actor%20Object%20Reference) (OtherComp :type Primitive%20Component%20Object%20Reference) (OtherBodyIndex :type Integer) (bFromSweep :type Boolean) (SweepResult :type Hit%20Result%20Structure%20%28by%20ref%29)))

(event OnSeePawn(PawnSensing)
  (params (Pawn :type Pawn%20Object%20Reference))
  (bind _ascharacter (Utilities|Casting|CastToCharacter Pawn))
  (Variables|Default|SetbIsInRange true)
  (Variables|Default|SetProjectileTarget (Variables|/Script/Engine.Character|GetCapsuleComponent _ascharacter))
  (Utilities|FlowControl|DoOnce false ; verhindert double fire wenn man den Aggro Bereich erneut betritt
    (:Completed
      (Utilities|Time|SetTimerbyEvent (delegate Custom|Fire) 1.0 true)
      (bind _returnvalue (Game|SpawnActorfromClass "/Game/Turret/ProjectilleTurret_BP.ProjectilleTurret_BP_C" (Math|Conversions|ToTransform(Vector) (Transformation|GetWorldLocation (Variables|Default|GetShootPoint))) "Undefined" 0 0))
      (Default|Follow _returnvalue (Variables|Default|GetProjectileTarget)))))

(event OnComponentEndOverlap(GTFO_Radius)
  (params (OverlappedComponent :type Primitive%20Component%20Object%20Reference) (OtherActor :type Actor%20Object%20Reference) (OtherComp :type Primitive%20Component%20Object%20Reference) (OtherBodyIndex :type Integer))
  (if true ; Tag nachträglich einfügen
    (Utilities|Casting|CastToCharacter OtherActor)
    (Variables|Default|SetbIsInRange false)
    (Utilities|Time|SetTimerbyEvent (delegate Custom|Fire) 0.0)
    (Utilities|FlowControl|DoOnce false) ; enters at Reset
  ))

(event Custom|Fire
  (bind _returnvalue (Game|SpawnActorfromClass "/Game/Turret/ProjectilleTurret_BP.ProjectilleTurret_BP_C" (Math|Conversions|ToTransform(Vector) (Transformation|GetWorldLocation (Variables|Default|GetShootPoint))) "Undefined" 0 0))
  (Default|Follow _returnvalue (Variables|Default|GetProjectileTarget)))

(event EventBeginPlay)

(event Game|Damage|EventAnyDamage
  (params (Damage :type Float%20%28single-precision%29) (DamageType :type Damage%20Type%20Object%20Reference) (InstigatedBy :type Controller%20Object%20Reference) (DamageCauser :type Actor%20Object%20Reference))
  (bind _output_get (Variables|Default|SetTurretHealth (- (Variables|Default|GetTurretHealth) Damage)))
  (bind _ashealth_bar (Utilities|Casting|CastToHealthBar (UserInterface|GetUserWidgetObject (Variables|Default|GetWidget))))
  (Default|Damage _ashealth_bar _output_get)
  (if (<= (Variables|Default|GetTurretHealth) 0.0)
    (Actor|DestroyActor)))

(fn ConstructionScript)