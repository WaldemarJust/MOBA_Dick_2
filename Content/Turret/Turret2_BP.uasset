(event OnSeePawn(PawnSensing)
  (params (Pawn :type Pawn%20Object%20Reference))
  (if (not (Actor|ActorHasTag "Team0"))
    (if (Variables|Default|GetbHasTarget)
      (if (<= (Transformation|GetDistanceTo Pawn) (Variables|Default|GetAttackRange))
        (Utilities|IsValid (stale _output_get) :!label _label
          (:Is%20Valid
            (Variables|Default|SetbHasTarget true)
            (Variables|Default|SetbIsInRange true)
            (Variables|Default|SetProjectileTarget (Variables|/Script/Engine.Character|GetCapsuleComponent (stale _output_get)))
            (bind _returnvalue (Game|SpawnActorfromClass "/Game/Turret/ProjectilleTurret_BP.ProjectilleTurret_BP_C" (Math|Conversions|ToTransform(Vector) (Transformation|GetWorldLocation (Variables|Default|GetShootPoint))) "Undefined" 0 0 0))
            (Default|Follow _returnvalue (Variables|Default|GetProjectileTarget)))
          (:Is%20Not%20Valid
            (Variables|Default|SetbHasTarget false :!label _label_2)
            (Variables|Default|SetbIsInRange false)))
        (else
          (Variables|Default|SetTarget 0)
          (goto _label_2)))
      (else
        (bind _ascharacter (Utilities|Casting|CastToCharacter Pawn))
        (bind _output_get (Variables|Default|SetTarget _ascharacter))
        (goto _label)))))

(event Game|Damage|EventAnyDamage
  (params (Damage :type Float%20%28single-precision%29) (DamageType :type Damage%20Type%20Object%20Reference) (InstigatedBy :type Controller%20Object%20Reference) (DamageCauser :type Actor%20Object%20Reference))
  (bind _output_get (Variables|Default|SetTurretHealth (- (Variables|Default|GetTurretHealth) Damage)))
  (bind _ashealth_bar (Utilities|Casting|CastToHealthBar (UserInterface|GetUserWidgetObject (Variables|Default|GetWidget))))
  (Default|Damage _ashealth_bar _output_get)
  (if (<= (Variables|Default|GetTurretHealth) 0.0)
    (Actor|DestroyActor)))

(fn ConstructionScript)