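; Base_BP is a destructible base actor that loses health when damaged.
; On any damage it subtracts the amount from its health and passes the new value to the HealthBar widget on its widget component.
; The actor destroys itself when health reaches zero or below, but only if the widget cast succeeds, since a failed cast stops the event first.
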(event Game|Damage|EventAnyDamage
  (params (Damage :type Float%20%28single-precision%29) (DamageType :type Damage%20Type%20Object%20Reference) (InstigatedBy :type Controller%20Object%20Reference) (DamageCauser :type Actor%20Object%20Reference))
  (bind _output_get (Variables|Default|SetBase0Health (- (Variables|Default|GetBase0Health) Damage)))
  (bind _ashealth_bar (Utilities|Casting|CastToHealthBar (UserInterface|GetUserWidgetObject (Variables|Default|GetWidget))))
  (Default|Damage _ashealth_bar _output_get)
  (if (<= (Variables|Default|GetBase0Health) 0.0)
    (Actor|DestroyActor)))

(fn ConstructionScript)